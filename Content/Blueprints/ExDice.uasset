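; ExDice is a dice actor Blueprint with a single CheckPlane function that probes the surface below it and launches its Box component.
; CheckPlane line-traces straight down on the Visibility channel, prints the hit actor's name, then applies an impulse to Box.
; The impulse adds the world-space impact point to a scaled actor up vector, so it varies with position.
; The event graph and construction script are empty, and nothing here calls CheckPlane.
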(fn `CheckPlane`
  (bind _outhit (`KismetSystemLibrary.LineTraceSingle` (`self.K2_GetActorLocation`) (`KismetMathLibrary.MakeVector` (.x (`self.K2_GetActorLocation`)) (.y (`self.K2_GetActorLocation`)) (- (.z (`self.K2_GetActorLocation`)) 10000.0)) "TraceTypeQuery1"))
  (bind (_bblockinghit _binitialoverlap _time _distance _location _impactpoint _normal _impactnormal _physmat _hitactor) (`GameplayStatics.BreakHitResult` _outhit))
  (`KismetSystemLibrary.PrintString` (`KismetSystemLibrary.GetDisplayName` _hitactor))
  (`PrimitiveComponent.AddImpulse` (`self.Box`) (+ _impactpoint (* (`self.GetActorUpVector`) 10000.0)) "None" false))

(fn `UserConstructionScript`)