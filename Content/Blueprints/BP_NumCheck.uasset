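; BP_NumCheck is a debug actor that probes which component faces up on each die, apparently to read rolled numbers.
; It enables player input on BeginPlay, and pressing 3 gathers every BP_ExDice actor tagged "Dice".
; For each die, a short downward Visibility trace runs from just above its location to that location.
; The die index, hit actor, hit component and component tags print on screen in debug colors.
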(event `self.ReceiveBeginPlay`
  (`self.EnableInput` (`GameplayStatics.GetPlayerController` 0)))

(event `Key|Three`
  (params (Key :type "Key Structure"))
  (:`Pressed`
    (bind _outactors (`GameplayStatics.GetAllActorsOfClassWithTag` "/Game/Blueprints/BP_ExDice.BP_ExDice_C" "Dice"))
    (for (_array_element _array_index) _outactors
      (`KismetSystemLibrary.PrintString` (`KismetStringLibrary.Conv_IntToString` _array_index) true true (struct :`G` 0.66 :`B` 1.0 :`A` 1.0) 10.0)
      (bind _returnvalue (`self.K2_GetActorLocation` _array_element))
      (bind _outhit (`KismetSystemLibrary.LineTraceSingle` :`Start` (+ _returnvalue (0.0 0.0 50.0)) :`End` _returnvalue :`TraceChannel` "TraceTypeQuery1" :`DrawDebugType` "ForDuration" :`TraceColor` (struct :`R` 1.0 :`B` 0.959337 :`A` 1.0)))
      (bind (_bblockinghit _binitialoverlap _time _distance _location _impactpoint _normal _impactnormal _physmat _hitactor _hitcomponent) (`GameplayStatics.BreakHitResult` _outhit))
      (`KismetSystemLibrary.PrintString` (`KismetSystemLibrary.GetDisplayName` _hitactor) true true (struct :`R` 1.0 :`G` 0.78409 :`A` 1.0) 10.0)
      (`KismetSystemLibrary.PrintString` (`KismetSystemLibrary.GetDisplayName` _hitcomponent) true true (struct :`R` 0.238418 :`B` 1.0 :`A` 1.0) 10.0)
      (for _array_element_2 (`ActorComponent.ComponentTags` _hitcomponent)
        (`KismetSystemLibrary.PrintString` (`KismetStringLibrary.Conv_NameToString` _array_element_2) true true (struct :`R` 1.0 :`A` 1.0) 10.0)))))

(fn `UserConstructionScript`)